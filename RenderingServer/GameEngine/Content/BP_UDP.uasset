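; Actor that links the game to a local process over UDP, exchanging JSON status messages and triggering a level sequence.
; On BeginPlay it opens loopback send and receive sockets, taking numeric ports from command-line arguments.
; Each received packet is parsed into GetData, then echoed back with the actor's rstatus field set.
; After replying it prints Cstatus, and a value of 10 plays the referenced sequence once through a DoOnce.
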(event OnReceivedBytes(UDP)
  (params (Bytes :type Array%20of%20Bytes) (IPAddress :type String))
  (bind _returnvalue (Class|MyBPJson|MyBytestoString Bytes))
  (bind _outjsonobject (Class|JsonBlueprintFunctionLibrary|FromString _returnvalue))
  (bind _outvalue (|GetJsonField _outjsonobject))
  (bind _output_get (Variables|Default|SetGetData _outvalue))
  (bind _returnvalue_2 (|SetJsonField _outjsonobject "rstatus" (Variables|Default|Getmyrstatus)))
  (if _returnvalue_2
    (bind (_outjsonstring _returnvalue_3) (Class|JsonBlueprintFunctionLibrary|ToString _outjsonobject))
    (if _returnvalue_3
      (bind _returnvalue_4 (Class|MyBPJson|MyStringtoBytes _outjsonstring))
      (Class|UDPComponent|EmitBytes (Variables|Default|GetUDP) _returnvalue_4)
      (Development|PrintString (Utilities|String|ToString(Integer) (.cstatus (Utilities|Struct|BreakMyUDPData _output_get))))
      (switch int (.cstatus (Utilities|Struct|BreakMyUDPData _output_get))
        (:10
          (Utilities|FlowControl|DoOnce false
            (:Completed
              (Sequencer|Player|Play (Variables|/Script/LevelSequence.LevelSequenceActor|GetSequencePlayer (Variables|Default|Getsequncer)) :!class /Script/MovieScene.MovieSceneSequencePlayer))))))))

(event EventBeginPlay
  (bind _returnvalue (Class|MyBPJson|MyGetCommandLine "portrecv"))
  (if (Class|KismetStringLibrary|IsNumeric _returnvalue)
    (Variables|Default|Setportrecv (Math|Conversions|ToInteger(Byte) _returnvalue)))
  (bind _returnvalue_2 (Class|MyBPJson|MyGetCommandLine "portsend"))
  (if (Class|KismetStringLibrary|IsNumeric _returnvalue_2)
    (Variables|Default|Setportsend (Math|Conversions|ToInteger(Byte) _returnvalue_2)))
  (Class|UDPComponent|OpenReceiveSocket (Variables|Default|GetUDP) "127.0.0.1" (Variables|Default|Getportrecv))
  (Class|UDPComponent|OpenSendSocket (Variables|Default|GetUDP) "127.0.0.1" (Variables|Default|Getportsend)))

(event Collision|EventActorBeginOverlap
  (params (OtherActor :type Actor%20Object%20Reference)))

(event EventTick
  (params (DeltaSeconds :type Float%20%28single-precision%29)))

(fn ConstructionScript)